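; BP_EngineStand is an engine stand actor that previews a DVSEngine component with a widget and a heat-reactive mesh.
; BeginPlay passes the engine component to W_EngineStandWidget and creates a dynamic material instance on the Cube mesh.
; Tick writes the engine's percent to overheat into that material's OverheatPercent parameter.
; The engine's start and stop events switch actor ticking on and off, so the material updates only while it runs.
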(event OnStartEngine(DVSEngine)
  (Actor|Tick|SetActorTickEnabled true))

(event OnStopEngine(DVSEngine)
  (Actor|Tick|SetActorTickEnabled false))

(event EventBeginPlay
  ;[1 0 0] For preview
  (bind _asw_engine_stand_widget (Utilities|Casting|CastToW_EngineStandWidget (UserInterface|GetWidget (Variables|Default|GetWidget)))
    (:then
      (Default|SetEngineComponent _asw_engine_stand_widget (Variables|Default|GetDVSEngine)))
    (:CastFailed
      _))
  (bind _returnvalue (Rendering|Material|CreateDynamicMaterialInstance (Variables|Default|GetCube) 0 0 "None" :!class /Script/Engine.PrimitiveComponent))
  (Variables|Default|SetMaterialEngine _returnvalue))

(event Collision|EventActorBeginOverlap
  (params (OtherActor :type Actor%20Object%20Reference)))

(event EventTick
  (params (DeltaSeconds :type Float%20%28single-precision%29))
  ;[1 0 0] For preview
  (bind _materialengine (Variables|Default|GetMaterialEngine)
    (:then
      (Rendering|Material|SetScalarParameterValue _materialengine "OverheatPercent" (Class|EngineComponent|GetPercenttoOverheat (Variables|Default|GetDVSEngine)) :!class /Script/Engine.MaterialInstanceDynamic))
    (:else)))

(fn ConstructionScript)